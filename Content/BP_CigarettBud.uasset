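; BP_CigarettBud is a health pickup that adds AddedHealth to the top-down player character on overlap with its Box.
; It casts the overlapping actor to BP_TopDownCharacterNew, raises Health, prints the result and destroys itself.
; If the gain would reach or exceed MaxHealth, it only prints "error" and stays in the world, so the inner clamp to MaxHealth is normally unreachable.
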(event `self.Box.OnComponentBeginOverlap`
  (params (OverlappedComponent :type "PrimitiveComponent Object Reference") (OtherActor :type "Actor Object Reference") (OtherComp :type "PrimitiveComponent Object Reference") (OtherBodyIndex :type Integer) (bFromSweep :type Boolean) (SweepResult :type "HitResult Structure (by ref)"))
  (bind _asbp_top_down_character_new (cast `/Game/TopDown/Blueprints/BP_TopDownCharacterNew` OtherActor))
  (if (>= (+ (`/Game/TopDown/Blueprints/BP_TopDownCharacterNew.Health` _asbp_top_down_character_new) (`self.addedHealth`)) (`/Game/TopDown/Blueprints/BP_TopDownCharacterNew.MaxHealth` _asbp_top_down_character_new))
    (`KismetSystemLibrary.PrintString` "error")
    (else
      (bind _health (`/Game/TopDown/Blueprints/BP_TopDownCharacterNew.Health` _asbp_top_down_character_new))
      (bind _maxhealth (`/Game/TopDown/Blueprints/BP_TopDownCharacterNew.MaxHealth` _asbp_top_down_character_new))
      (if (> _health _maxhealth)
        (bind _output_get (set `/Game/TopDown/Blueprints/BP_TopDownCharacterNew.Health` _maxhealth _asbp_top_down_character_new))
        (`KismetSystemLibrary.PrintString` (`KismetStringLibrary.Conv_DoubleToString` _output_get))
        (else
          (bind _output_get_2 (set `/Game/TopDown/Blueprints/BP_TopDownCharacterNew.Health` (+ _health (`self.addedHealth`)) _asbp_top_down_character_new))
          (`KismetSystemLibrary.PrintString` (`KismetStringLibrary.Conv_DoubleToString` _output_get_2))))
      (`self.K2_DestroyActor`))))

(fn `UserConstructionScript`)