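; BP_Cat is a guard-like hazard that ends the level when its line of sight catches the player character.
; On BeginPlay it starts the LineOfSight component's traces and vision mesh, caches the player, and starts a looping timer that turns the cat by a random yaw.
; When the sight overlap hits the player, it meows, teleports to DestLocation, sounds an alarm, prints a loss message and restarts the level after a delay.
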(event `self.ReceiveBeginPlay`
  (bind _lineofsight (`self.LineOfSight`))
  (`LineOfSightComponent.StartLineTrace` _lineofsight "TraceTypeQuery1" 60)
  (`LineOfSightComponent.StartBuildMesh` _lineofsight)
  (bind _asbp_top_down_character_new (cast `/Game/TopDown/Blueprints/BP_TopDownCharacterNew` (`GameplayStatics.GetPlayerPawn` 0)))
  (set `self.As BP Top Down Character New` _asbp_top_down_character_new)
  (`KismetSystemLibrary.K2_SetTimerDelegate` (delegate `TurnRandomly`) 3.0 true))

(event `TurnRandomly`
  (`self.K2_AddActorWorldRotation` (`KismetMathLibrary.MakeRotator` 0.0 0.0 (`KismetMathLibrary.RandomFloatInRange` 0.0 180.0))))

(event `self.LineOfSight.BeginOverlap`
  (params (Hit :type "HitResult Structure (by ref)"))
  (if (== (`.HitActor` (`GameplayStatics.BreakHitResult` Hit)) (`self.As BP Top Down Character New`))
    (`GameplayStatics.PlaySound2D` "/Game/Sounds/SC_CatMeow.SC_CatMeow" 1.0 1.0 0.0 null null)
    (`self.K2_TeleportTo` (`self.Dest Location`))
    (`GameplayStatics.PlaySound2D` "/Game/Sounds/SC_CaughtAlarm.SC_CaughtAlarm" 1.0 1.0 0.0 null null)
    (`KismetSystemLibrary.PrintString` "You lost")
    (`KismetSystemLibrary.Delay` 2.0)
    (`KismetSystemLibrary.ExecuteConsoleCommand` "RestartLevel" null)))

(fn `UserConstructionScript`)