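; Generic AI controller that runs BT_AI, moves its BP_AI pawn along a level spline and tracks sighted actors.
; After a short delay it takes the first BP_Spline and derives travel duration from spline length and max walk speed.
; A timeline scaled to that duration issues MoveToLocation along the spline every update.
; Sight perception sets the blackboard Target Actor, while sight loss or other senses clear it.
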(event `self.ReceiveBeginPlay`
  (`self.RunBehaviorTree` "/Game/AI/BT_AI.BT_AI")
  (`KismetSystemLibrary.Delay` 0.2)
  (`|ExecutionSequence`
    (:`then_0`
      (bind _outactors (`GameplayStatics.GetAllActorsOfClass` "/Game/AI/BP_Spline.BP_Spline_C"))
      (set `self.SplineReference` (`|GetArrayItem` _outactors)))
    (:`then_1`
      (bind _asbp_ai (cast `/Game/AI/BP_AI` (`self.K2_GetPawn`)))
      (set `self.Duration` (/ (`SplineComponent.GetSplineLength` (`/Game/AI/BP_Spline.Spline` (`self.SplineReference`))) (`MovementComponent.GetMaxSpeed` (`Character.CharacterMovement` _asbp_ai)))))
    (:`then_2`
      (`self.Run`))))

(event `Run`
  (`TimelineComponent.SetPlayRate` (`self.MoveTimeline`) (/ 1.0 (`self.Duration`)))
  (bind (_direction _alpha) (`Timeline|MoveTimeline`)
    (:`Update`
      (set `self.Alpha` _alpha)
      (`self.MoveToLocation` (`SplineComponent.GetLocationAtDistanceAlongSpline` (`/Game/AI/BP_Spline.Spline` (`self.SplineReference`)) (`KismetMathLibrary.Lerp` 0.0 (`SplineComponent.GetSplineLength` (`/Game/AI/BP_Spline.Spline` (`self.SplineReference`))) (`self.Alpha`)) "World") -1.0 true true false true null))))

(event `self.AIPerception.OnTargetPerceptionUpdated`
  (params (Actor :type "Actor Object Reference") (Stimulus :type "AIStimulus Structure"))
  ;[1 1 1] Detect and chase target
  (bind _returnvalue (`AIPerceptionSystem.GetSenseClassForStimulus` Stimulus))
  (if (== _returnvalue "/Script/AIModule.AISense_Sight")
    (if (`.bSuccessfullySensed` (break `AIStimulus` Stimulus))
      (`BlackboardComponent.SetValueAsObject` (`AIBlueprintHelperLibrary.GetBlackboard` null) "Target Actor" Actor)
      (else
        (`BlackboardComponent.SetValueAsObject` (`AIBlueprintHelperLibrary.GetBlackboard` null) "Target Actor" null :!label _label)))
    (else
      (goto _label))))

(fn `UserConstructionScript`)