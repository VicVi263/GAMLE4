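; BP_Water is a water hazard that makes the player lose and restarts the level on contact.
; It caches the player pawn as BP_TopDownCharacterNew on BeginPlay and compares it against actors that begin overlapping its Sphere.
; On a match it plays a fire sizzle sound, prints a loss message, waits briefly, then runs the RestartLevel console command between disable and enable input calls.
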(event `self.ReceiveBeginPlay`
  (bind _asbp_top_down_character_new (cast `/Game/TopDown/Blueprints/BP_TopDownCharacterNew` (`GameplayStatics.GetPlayerPawn` 0)))
  (set `self.As BP Top Down Character New` _asbp_top_down_character_new))

(event `self.Sphere.OnComponentBeginOverlap`
  (params (OverlappedComponent :type "PrimitiveComponent Object Reference") (OtherActor :type "Actor Object Reference") (OtherComp :type "PrimitiveComponent Object Reference") (OtherBodyIndex :type Integer) (bFromSweep :type Boolean) (SweepResult :type "HitResult Structure (by ref)"))
  (if (== (`self.As BP Top Down Character New`) OtherActor)
    (`GameplayStatics.PlaySound2D` "/Game/Sounds/SC_FireSizzle.SC_FireSizzle" 1.0 1.0 0.0 null null)
    (`KismetSystemLibrary.PrintString` "You lost")
    (`KismetSystemLibrary.Delay` 1.0)
    (`self.DisableInput` null)
    (`KismetSystemLibrary.ExecuteConsoleCommand` "RestartLevel" null)
    (`self.EnableInput` null)))

(fn `UserConstructionScript`)