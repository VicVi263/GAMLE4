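; BP_WoodChip is a wood chip pickup that the top-down player character collects by walking into it.
; On BeginPlay it caches the player character; a Box overlap sets that character's HasWoodChip flag if not already set.
; Collection plays a fire-light sound and hides the sphere, spotlight and box, then shows them again after a short delay.
; Only visibility toggles, with collision left unchanged.
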(event `self.ReceiveBeginPlay`
  (bind _asbp_top_down_character_new (cast `/Game/TopDown/Blueprints/BP_TopDownCharacterNew` (`GameplayStatics.GetPlayerPawn` 0)))
  (set `self.As BP Top Down Character New` _asbp_top_down_character_new))

(event `self.Box.OnComponentBeginOverlap`
  (params (OverlappedComponent :type "PrimitiveComponent Object Reference") (OtherActor :type "Actor Object Reference") (OtherComp :type "PrimitiveComponent Object Reference") (OtherBodyIndex :type Integer) (bFromSweep :type Boolean) (SweepResult :type "HitResult Structure (by ref)"))
  (bind _as_bp_top_down_character_new (`self.As BP Top Down Character New`))
  (if (== OtherActor _as_bp_top_down_character_new)
    (if (not (`/Game/TopDown/Blueprints/BP_TopDownCharacterNew.bHasWoodChip` _as_bp_top_down_character_new))
      (set `/Game/TopDown/Blueprints/BP_TopDownCharacterNew.bHasWoodChip` true _as_bp_top_down_character_new)
      (`SceneComponent.SetVisibility` (`self.Sphere`) false false)
      (`SceneComponent.SetVisibility` (`self.SpotLight`) false false)
      (`SceneComponent.SetVisibility` (`self.Box`) false false)
      (`GameplayStatics.PlaySound2D` "/Game/Sounds/SC_FireLight.SC_FireLight" 1.0 1.0 0.0 null null)
      (`KismetSystemLibrary.Delay` 5.0)
      (`SceneComponent.SetVisibility` (`self.Sphere`) true false)
      (`SceneComponent.SetVisibility` (`self.SpotLight`) true false)
      (`SceneComponent.SetVisibility` (`self.Box`) true false))))

(fn `UserConstructionScript`)