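; BP_WindNegative is a box volume that marks an area where the top-down player character is not affected as being inside wind.
; On BeginPlay it caches the player pawn as BP_TopDownCharacterNew and stops its Audio component.
; When that character enters the Box, IsInsideWind is cleared.
; Leaving always sets the flag to true, without checking for a surrounding wind area.
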(event `self.ReceiveBeginPlay`
  (bind _asbp_top_down_character_new (cast `/Game/TopDown/Blueprints/BP_TopDownCharacterNew` (`GameplayStatics.GetPlayerPawn` 0)))
  (set `self.As BP Top Down Character New` _asbp_top_down_character_new)
  (`AudioComponent.Stop` (`self.Audio`)))

(event `self.Box.OnComponentBeginOverlap`
  (params (OverlappedComponent :type "PrimitiveComponent Object Reference") (OtherActor :type "Actor Object Reference") (OtherComp :type "PrimitiveComponent Object Reference") (OtherBodyIndex :type Integer) (bFromSweep :type Boolean) (SweepResult :type "HitResult Structure (by ref)"))
  (bind _as_bp_top_down_character_new (`self.As BP Top Down Character New`))
  (if (== _as_bp_top_down_character_new OtherActor)
    (set `/Game/TopDown/Blueprints/BP_TopDownCharacterNew.bIsInsideWind` false _as_bp_top_down_character_new)))

(event `self.Box.OnComponentEndOverlap`
  (params (OverlappedComponent :type "PrimitiveComponent Object Reference") (OtherActor :type "Actor Object Reference") (OtherComp :type "PrimitiveComponent Object Reference") (OtherBodyIndex :type Integer))
  (bind _as_bp_top_down_character_new (`self.As BP Top Down Character New`))
  (if (== _as_bp_top_down_character_new OtherActor)
    (set `/Game/TopDown/Blueprints/BP_TopDownCharacterNew.bIsInsideWind` true _as_bp_top_down_character_new)))

(fn `UserConstructionScript`)