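; BP_enemy is a patrolling AI enemy that catches the top-down player on sight and restarts the level.
; When activated, it loops AI MoveTo between a start and end actor, pausing briefly at each.
; A LineOfSight component runs line traces and builds a mesh from BeginPlay.
; When its overlap hits the cached player character, it plays death and alarm sounds, then restarts the level after a delay.
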(event `self.ReceiveBeginPlay`
  (bind _lineofsight (`self.LineOfSight`))
  (`self.BackAndForth`)
  (`LineOfSightComponent.StartLineTrace` _lineofsight "TraceTypeQuery1" 60)
  (`LineOfSightComponent.StartBuildMesh` _lineofsight)
  (bind _asbp_top_down_character_new (cast `/Game/TopDown/Blueprints/BP_TopDownCharacterNew` (`GameplayStatics.GetPlayerPawn` 0)))
  (set `self.As BP Top Down Character New` _asbp_top_down_character_new))

(event `BackAndForth`
  (bind _startinglocation (`self.StartingLocation`))
  ;[1 1 1] Moves the Ai back and forth two positions
  (if (`self.activate`)
    (`/Engine/EditorBlueprintResources/StandardMacros.IsValid` _startinglocation
      (:`Is Valid`
        (`|AIMoveTo` self (`self.K2_GetActorLocation` _startinglocation) null 5.0 true
          (:`OnSuccess`
            (`KismetSystemLibrary.Delay` 1.5)
            (`|AIMoveTo` self (`self.K2_GetActorLocation` (`self.EndLocation`)) null 5.0 true
              (:`OnSuccess`
                (`KismetSystemLibrary.Delay` 1.5)
                (`self.BackAndForth`))))
          (:`OnFail`
            (`KismetSystemLibrary.PrintString` "Fail")))))))

(event `self.LineOfSight.BeginOverlap`
  (params (Hit :type "HitResult Structure (by ref)"))
  (if (== (`.HitActor` (`GameplayStatics.BreakHitResult` Hit)) (`self.As BP Top Down Character New`))
    (`GameplayStatics.PlaySound2D` "/Game/Sounds/SC_Death.SC_Death" 1.0 1.0 0.0 null null)
    (`GameplayStatics.PlaySound2D` "/Game/Sounds/SC_CaughtAlarm.SC_CaughtAlarm" 1.0 1.0 0.0 null null)
    (`KismetSystemLibrary.PrintString` "You lost")
    (`KismetSystemLibrary.Delay` 2.0)
    (`KismetSystemLibrary.ExecuteConsoleCommand` "RestartLevel" null)))

(fn `UserConstructionScript`)